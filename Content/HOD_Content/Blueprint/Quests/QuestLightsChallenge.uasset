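; Quest trigger that issues a one-time, timed challenge, apparently about lights, with viewer count as the stake.
; When the player enters the box, it generates and stores a message owner, then posts event messages through HODGameInstance.
; After a delay, a true StillOut flag awards viewers and posts completion messages under that owner.
; A Lose event, not called within this graph, deducts viewers and posts exit messages.
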(event OnComponentBeginOverlap(Box)
  (params (OverlappedComponent :type Primitive%20Component%20Object%20Reference) (OtherActor :type Actor%20Object%20Reference) (OtherComp :type Primitive%20Component%20Object%20Reference) (OtherBodyIndex :type Integer) (bFromSweep :type Boolean) (SweepResult :type Hit%20Result%20Structure%20%28by%20ref%29))
  (bind _returnvalue (Game|GetGameInstance))
  (bind _returnvalue_2 (Game|GetGameInstance))
  (bind _ashodgame_instance (Utilities|Casting|CastToHODGameInstance _returnvalue_2))
  (bind _ashodgame_instance_2 (Utilities|Casting|CastToHODGameInstance _returnvalue))
  (Utilities|Casting|CastToHOD_Player OtherActor)
  (Utilities|FlowControl|DoOnce false
    (:Completed
      (Default|GenerateOwner _ashodgame_instance)
      (Variables|Default|SetStoredUser (Variables|/Game/HOD_Content/Blueprint/GameInstance/HODGameInstance.HODGameInstance_C|GetOwner _ashodgame_instance))
      (Variables|/Game/HOD_Content/Blueprint/GameInstance/HODGameInstance.HODGameInstance_C|SetStoredOwner _ashodgame_instance true)
      (Variables|/Game/HOD_Content/Blueprint/GameInstance/HODGameInstance.HODGameInstance_C|SetSpecialMessage _ashodgame_instance true)
      (Variables|/Game/HOD_Content/Blueprint/GameInstance/HODGameInstance.HODGameInstance_C|SetMensajesContext _ashodgame_instance (Variables|Default|GetMessagesEvento))
      (Variables|/Game/HOD_Content/Blueprint/GameInstance/HODGameInstance.HODGameInstance_C|SetContextTime _ashodgame_instance (Variables|Default|GetSpawnTime))
      (Utilities|FlowControl|Delay (Variables|Default|GetCheckTime))
      (if (Variables|Default|GetStillOut)
        (Default|AddViewers (.AsHODGame%20Instance (Utilities|Casting|CastToHODGameInstance (Game|GetGameInstance))) (Variables|Default|GetViewers))
        (Variables|/Game/HOD_Content/Blueprint/GameInstance/HODGameInstance.HODGameInstance_C|SetSpecialMessage _ashodgame_instance_2 true)
        (Variables|/Game/HOD_Content/Blueprint/GameInstance/HODGameInstance.HODGameInstance_C|SetMensajesContext _ashodgame_instance_2 (Variables|Default|GetCompleteEvent))
        (Variables|/Game/HOD_Content/Blueprint/GameInstance/HODGameInstance.HODGameInstance_C|SetContextTime _ashodgame_instance_2 (Variables|Default|GetSpawnTime))
        (Variables|/Game/HOD_Content/Blueprint/GameInstance/HODGameInstance.HODGameInstance_C|SetOwner _ashodgame_instance_2 (Variables|Default|GetStoredUser))
        (Variables|/Game/HOD_Content/Blueprint/GameInstance/HODGameInstance.HODGameInstance_C|SetStoredOwner _ashodgame_instance_2 true)))))

(event Custom|Lose
  (bind _returnvalue (Game|GetGameInstance))
  (bind _ashodgame_instance (Utilities|Casting|CastToHODGameInstance _returnvalue))
  (Default|AddViewers (.AsHODGame%20Instance (Utilities|Casting|CastToHODGameInstance (Game|GetGameInstance))) (* (Variables|Default|GetViewers) -1))
  (Variables|/Game/HOD_Content/Blueprint/GameInstance/HODGameInstance.HODGameInstance_C|SetSpecialMessage _ashodgame_instance true)
  (Variables|/Game/HOD_Content/Blueprint/GameInstance/HODGameInstance.HODGameInstance_C|SetMensajesContext _ashodgame_instance (Variables|Default|GetExitEvent))
  (Variables|/Game/HOD_Content/Blueprint/GameInstance/HODGameInstance.HODGameInstance_C|SetContextTime _ashodgame_instance (Variables|Default|GetSpawnTime))
  (Variables|/Game/HOD_Content/Blueprint/GameInstance/HODGameInstance.HODGameInstance_C|SetOwner _ashodgame_instance (Variables|Default|GetStoredUser))
  (Variables|/Game/HOD_Content/Blueprint/GameInstance/HODGameInstance.HODGameInstance_C|SetStoredOwner _ashodgame_instance true))

(fn ConstructionScript)