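; A quest trigger for finding an object, which reacts once when the player overlaps its box while it is activated.
; After a configurable delay, it adds viewers through the game instance and flags a special message.
; It also passes the completion context text, display time and stored owner to the game instance, reusing the delay value as the display time.
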(event OnComponentBeginOverlap(Box)
  (params (OverlappedComponent :type Primitive%20Component%20Object%20Reference) (OtherActor :type Actor%20Object%20Reference) (OtherComp :type Primitive%20Component%20Object%20Reference) (OtherBodyIndex :type Integer) (bFromSweep :type Boolean) (SweepResult :type Hit%20Result%20Structure%20%28by%20ref%29))
  (bind _returnvalue (Game|GetGameInstance))
  (bind _ashodgame_instance (Utilities|Casting|CastToHODGameInstance _returnvalue))
  (if (Variables|Default|GetActivated)
    (Utilities|Casting|CastToHOD_Player OtherActor)
    (Utilities|FlowControl|DoOnce false
      (:Completed
        (Utilities|FlowControl|Delay (Variables|Default|GetTimeToShow))
        (Default|AddViewers _ashodgame_instance (Variables|Default|GetViewers))
        (Variables|/Game/HOD_Content/Blueprint/GameInstance/HODGameInstance.HODGameInstance_C|SetSpecialMessage _ashodgame_instance true)
        (Variables|/Game/HOD_Content/Blueprint/GameInstance/HODGameInstance.HODGameInstance_C|SetMensajesContext _ashodgame_instance (Variables|Default|GetCompleteEvent))
        (Variables|/Game/HOD_Content/Blueprint/GameInstance/HODGameInstance.HODGameInstance_C|SetContextTime _ashodgame_instance (Variables|Default|GetTimeToShow))
        (Variables|/Game/HOD_Content/Blueprint/GameInstance/HODGameInstance.HODGameInstance_C|SetOwner _ashodgame_instance (Variables|Default|GetOwnerStored))
        (Variables|/Game/HOD_Content/Blueprint/GameInstance/HODGameInstance.HODGameInstance_C|SetStoredOwner _ashodgame_instance true)))))

(fn ConstructionScript)