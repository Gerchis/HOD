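; One-shot trigger volume for a crouch challenge issued through the game's viewer chat messages.
; When the player overlaps the box, it resets their crouch counter, generates and stores a message owner, and posts the challenge through the GameInstance.
; After a timed delay it compares the counter to the required count and posts a success or failure message from that owner.
; Success also shows an Alert widget and plays viewer animations.
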(event OnComponentBeginOverlap(Box)
  (params (OverlappedComponent :type Primitive%20Component%20Object%20Reference) (OtherActor :type Actor%20Object%20Reference) (OtherComp :type Primitive%20Component%20Object%20Reference) (OtherBodyIndex :type Integer) (bFromSweep :type Boolean) (SweepResult :type Hit%20Result%20Structure%20%28by%20ref%29))
  (bind _returnvalue (Game|GetGameInstance))
  (bind _returnvalue_2 (Game|GetGameInstance))
  (bind _returnvalue_3 (Game|GetGameInstance))
  (bind _returnvalue_4 (Game|GetGameInstance))
  (bind _ashodgame_instance (Utilities|Casting|CastToHODGameInstance _returnvalue_2))
  (bind _ashodgame_instance_2 (Utilities|Casting|CastToHODGameInstance _returnvalue_4))
  (bind _ashodgame_instance_3 (Utilities|Casting|CastToHODGameInstance _returnvalue_3))
  (bind _ashodgame_instance_4 (Utilities|Casting|CastToHODGameInstance _returnvalue))
  (bind _chatfullscreen (Variables|/Game/HOD_Content/Blueprint/GameInstance/HODGameInstance.HODGameInstance_C|GetChatFullscreen _ashodgame_instance))
  (Utilities|Casting|CastToHOD_Player OtherActor)
  (Utilities|FlowControl|DoOnce false
    (:Completed
      (Variables|/Game/HOD_Content/Blueprint/Character/HOD_Player.HOD_Player_C|SetCrouchTime (.AsHOD%20Player (Utilities|Casting|CastToHOD_Player (Game|GetPlayerCharacter 0))) 0)
      (Default|GenerateOwner _ashodgame_instance_3)
      (Variables|Default|SetStoredOwner (Variables|/Game/HOD_Content/Blueprint/GameInstance/HODGameInstance.HODGameInstance_C|GetOwner _ashodgame_instance_3))
      (Variables|/Game/HOD_Content/Blueprint/GameInstance/HODGameInstance.HODGameInstance_C|SetStoredOwner _ashodgame_instance_3 true)
      (Variables|/Game/HOD_Content/Blueprint/GameInstance/HODGameInstance.HODGameInstance_C|SetSpecialMessage _ashodgame_instance_3 true)
      (Variables|/Game/HOD_Content/Blueprint/GameInstance/HODGameInstance.HODGameInstance_C|SetMensajesContext _ashodgame_instance_3 (Variables|Default|GetMessagesEvento))
      (Variables|/Game/HOD_Content/Blueprint/GameInstance/HODGameInstance.HODGameInstance_C|SetContextTime _ashodgame_instance_3 (Variables|Default|GetSpawnTime))
      (Utilities|FlowControl|Delay (Variables|Default|GetCheckTime))
      (if (< (Variables|Default|GetCrouchTimes) (Variables|/Game/HOD_Content/Blueprint/Character/HOD_Player.HOD_Player_C|GetCrouchTime (.AsHOD%20Player (Utilities|Casting|CastToHOD_Player (Game|GetPlayerCharacter 0)))))
        (Variables|/Game/HOD_Content/Blueprint/GameInstance/HODGameInstance.HODGameInstance_C|SetSpecialMessage _ashodgame_instance_4 true)
        (Variables|/Game/HOD_Content/Blueprint/GameInstance/HODGameInstance.HODGameInstance_C|SetMensajesContext _ashodgame_instance_4 (Variables|Default|GetCompleteEvent))
        (Variables|/Game/HOD_Content/Blueprint/GameInstance/HODGameInstance.HODGameInstance_C|SetContextTime _ashodgame_instance_4 (Variables|Default|GetSpawnTime))
        (Variables|/Game/HOD_Content/Blueprint/GameInstance/HODGameInstance.HODGameInstance_C|SetOwner _ashodgame_instance_4 (Variables|Default|GetStoredOwner))
        (Variables|/Game/HOD_Content/Blueprint/GameInstance/HODGameInstance.HODGameInstance_C|SetStoredOwner _ashodgame_instance_4 true)
        (bind _returnvalue_5 (UserInterface|CreateWidget "/Game/HOD_Content/Blueprint/ChatHUD/Alert.Alert_C"))
        (UserInterface|Viewport|AddtoViewport _returnvalue_5 0)
        (Default|PlayViewersAnim _returnvalue_5)
        (UserInterface|Animation|PlayAnimation _chatfullscreen (Variables|/Game/HOD_Content/Blueprint/ChatHUD/FullscreenGame.FullscreenGame_C|GetViewersAnim _chatfullscreen) 0.0 1 "Forward" 0.5 false)
        (else
          (Variables|/Game/HOD_Content/Blueprint/GameInstance/HODGameInstance.HODGameInstance_C|SetSpecialMessage _ashodgame_instance_2 true)
          (Variables|/Game/HOD_Content/Blueprint/GameInstance/HODGameInstance.HODGameInstance_C|SetMensajesContext _ashodgame_instance_2 (Variables|Default|GetFailEvent))
          (Variables|/Game/HOD_Content/Blueprint/GameInstance/HODGameInstance.HODGameInstance_C|SetContextTime _ashodgame_instance_2 (Variables|Default|GetSpawnTime))
          (Variables|/Game/HOD_Content/Blueprint/GameInstance/HODGameInstance.HODGameInstance_C|SetOwner _ashodgame_instance_2 (Variables|Default|GetStoredOwner))
          (Variables|/Game/HOD_Content/Blueprint/GameInstance/HODGameInstance.HODGameInstance_C|SetStoredOwner _ashodgame_instance_2 true))))))

(fn ConstructionScript)