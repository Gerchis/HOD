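; FindTrigger is a quest trigger volume that activates its referenced Finding when the player enters it.
; The Box overlap filters for HOD_Player and passes through a DoOnce, so it fires only once.
; It then calls GenerateGameMessage on HODGameInstance, flags the message as special and hands over its event message content and display timing from MessagesEvento and SpawnTime.
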(event OnComponentBeginOverlap(Box)
  (params (OverlappedComponent :type Primitive%20Component%20Object%20Reference) (OtherActor :type Actor%20Object%20Reference) (OtherComp :type Primitive%20Component%20Object%20Reference) (OtherBodyIndex :type Integer) (bFromSweep :type Boolean) (SweepResult :type Hit%20Result%20Structure%20%28by%20ref%29))
  (bind _returnvalue (Game|GetGameInstance))
  (bind _ashodgame_instance (Utilities|Casting|CastToHODGameInstance _returnvalue))
  (Utilities|Casting|CastToHOD_Player OtherActor)
  (Utilities|FlowControl|DoOnce false
    (:Completed
      (Variables|/Game/HOD_Content/Blueprint/Quests/FindObjectTrigger.FindObjectTrigger_C|SetActivated (Variables|Default|GetFinding) true)
      (Default|GenerateGameMessage _ashodgame_instance true)
      (Variables|/Game/HOD_Content/Blueprint/GameInstance/HODGameInstance.HODGameInstance_C|SetSpecialMessage _ashodgame_instance true)
      (Variables|/Game/HOD_Content/Blueprint/GameInstance/HODGameInstance.HODGameInstance_C|SetMensajesContext _ashodgame_instance (Variables|Default|GetMessagesEvento))
      (Variables|/Game/HOD_Content/Blueprint/GameInstance/HODGameInstance.HODGameInstance_C|SetContextTime _ashodgame_instance (Variables|Default|GetSpawnTime)))))

(fn ConstructionScript)