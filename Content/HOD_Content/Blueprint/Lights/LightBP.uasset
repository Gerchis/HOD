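; Switchable light fixture actor whose fluorescent mesh, point light and spot light turn on and off together.
; The construction script applies both light intensities and previews the OnOff state through light visibility and a dynamic material instance.
; BeginPlay creates any missing on or off material instance, then calls TurnOn if OnOff is set.
; TurnOn and TurnOff toggle the Lights component and its children, swap the mesh material and update OnOff.
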(event Custom|TurnOff
  (Rendering|SetVisibility (Variables|Default|GetLights) false true)
  (Rendering|Material|SetMaterial (Variables|Default|GetStaticMesh) 0 (Variables|Default|GetOffMAT))
  (Variables|Default|SetOn_Off false))

(event Custom|TurnOn
  (Rendering|SetVisibility (Variables|Default|GetLights) true true)
  (Rendering|Material|SetMaterial (Variables|Default|GetStaticMesh) 0 (Variables|Default|GetOnMAT))
  (Variables|Default|SetOn_Off true))

(event EventBeginPlay
  (Variables|Default|GetOnMAT
    (:then
      (bind _offmat (Variables|Default|GetOffMAT)
        (:then
          (Rendering|Material|SetMaterial (Variables|Default|GetStaticMesh) 0 _offmat)
          (if (Variables|Default|GetOn_Off)
            (CallFunction|Turnon)))
        (:else
          (bind _returnvalue (Rendering|Material|CreateDynamicMaterialInstance (Variables|Default|GetStaticMesh) 0 "/Game/PropsFBX/Fluorescente/FluorescenteApagado_Inst.FluorescenteApagado_Inst" "None" :!class /Script/Engine.PrimitiveComponent))
          (Variables|Default|SetOffMAT _returnvalue)
          (if (Variables|Default|GetOn_Off)
            (CallFunction|Turnon)))))
    (:else
      (bind _returnvalue_2 (Rendering|Material|CreateDynamicMaterialInstance (Variables|Default|GetStaticMesh) 0 "/Game/PropsFBX/Fluorescente/FluorescenteEncendido_Inst.FluorescenteEncendido_Inst" "None" :!class /Script/Engine.PrimitiveComponent))
      (Variables|Default|SetOnMAT _returnvalue_2)
      (bind _offmat_2 (Variables|Default|GetOffMAT)
        (:then
          (Rendering|Material|SetMaterial (Variables|Default|GetStaticMesh) 0 _offmat_2)
          (if (Variables|Default|GetOn_Off)
            (CallFunction|Turnon)))
        (:else
          (bind _returnvalue_3 (Rendering|Material|CreateDynamicMaterialInstance (Variables|Default|GetStaticMesh) 0 "/Game/PropsFBX/Fluorescente/FluorescenteApagado_Inst.FluorescenteApagado_Inst" "None" :!class /Script/Engine.PrimitiveComponent))
          (Variables|Default|SetOffMAT _returnvalue_3)
          (if (Variables|Default|GetOn_Off)
            (CallFunction|Turnon)))))))

(fn ConstructionScript
  (Rendering|Components|Light|SetIntensity (Variables|Default|GetPointLight) (Variables|Default|GetLightStrenghtPoint))
  (Rendering|Components|Light|SetIntensity (Variables|Default|GetSpotLight) (Variables|Default|GetLightStrengthSpot))
  (if (Variables|Default|GetOn_Off)
    (Rendering|SetVisibility (Variables|Default|GetLights) true true)
    (bind _returnvalue (Rendering|Material|CreateDynamicMaterialInstance (Variables|Default|GetStaticMesh) 0 "/Game/PropsFBX/Fluorescente/FluorescenteEncendido_Inst.FluorescenteEncendido_Inst" "None" :!class /Script/Engine.PrimitiveComponent))
    (Variables|Default|SetOnMAT _returnvalue)
    (else
      (Rendering|SetVisibility (Variables|Default|GetLights) false true)
      (bind _returnvalue_2 (Rendering|Material|CreateDynamicMaterialInstance (Variables|Default|GetStaticMesh) 0 "/Game/PropsFBX/Fluorescente/FluorescenteApagado_Inst.FluorescenteApagado_Inst" "None" :!class /Script/Engine.PrimitiveComponent))
      (Variables|Default|SetOffMAT _returnvalue_2))))