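; PlomosLuz is an interactable power switch that turns on the level's lights once.
; Entering its Interact volume registers it as the HOD_Player's interact target and glows both interruptor components; leaving removes the glow but not the reference.
; InteractwithActor runs through a DoOnce, plays a button sound, then calls TurnOn on every LightBP and SparklingLightBP found with GetAllActorsOfClass.
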(event OnComponentBeginOverlap(Interact)
  (params (OverlappedComponent :type Primitive%20Component%20Object%20Reference) (OtherActor :type Actor%20Object%20Reference) (OtherComp :type Primitive%20Component%20Object%20Reference) (OtherBodyIndex :type Integer) (bFromSweep :type Boolean) (SweepResult :type Hit%20Result%20Structure%20%28by%20ref%29))
  (bind _ashod_player (Utilities|Casting|CastToHOD_Player OtherActor))
  (Variables|/Game/HOD_Content/Blueprint/Character/HOD_Player.HOD_Player_C|SetInteract _ashod_player self)
  (Default|ActivateGlow _ashod_player (Utilities|Array|MakeArray (Variables|Default|GetInterruptorOff) (Variables|Default|GetInterruptorOn))))

(event OnComponentEndOverlap(Interact)
  (params (OverlappedComponent :type Primitive%20Component%20Object%20Reference) (OtherActor :type Actor%20Object%20Reference) (OtherComp :type Primitive%20Component%20Object%20Reference) (OtherBodyIndex :type Integer))
  (bind _ashod_player (Utilities|Casting|CastToHOD_Player OtherActor))
  (Default|DesactivateGlow _ashod_player (Utilities|Array|MakeArray (Variables|Default|GetInterruptorOff) (Variables|Default|GetInterruptorOn))))

(event EventInteractwithActor
  (Utilities|FlowControl|DoOnce false
    (:Completed
      (Audio|PlaySoundatLocation "/Game/HorrorEngine/Audio/Button/ButtonOn02.ButtonOn02" (Transformation|GetActorLocation) "0, 0, 0" 1.0 1.0 0.0 0 0 0)
      (bind _outactors (Actor|GetAllActorsOfClass "/Game/HOD_Content/Blueprint/Lights/LightBP.LightBP_C"))
      (for _array_element _outactors
        (Default|Turnon _array_element))
      (bind _outactors_2 (Actor|GetAllActorsOfClass "/Game/HOD_Content/Blueprint/Lights/SparklingLightBP.SparklingLightBP_C"))
      (for _array_element_2 _outactors_2
        (Default|Turnon _array_element_2)))))

(fn ConstructionScript)