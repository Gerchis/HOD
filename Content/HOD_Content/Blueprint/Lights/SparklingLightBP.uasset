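; Flickering fluorescent light actor that blinks a spotlight and swaps its mesh between lit and unlit materials.
; The construction script applies intensity and initial visibility, and BeginPlay fills in missing dynamic material instances, then applies the unlit one.
; While OnOff is true, Tick drives a DoOnce, random Delay and FlipFlop loop that alternates both states.
; TurnOn and TurnOff only set that flag, so stopping can leave the light lit.
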(event Custom|TurnOff
  (Variables|Default|SetOn_Off false))

(event Custom|TurnOn
  (Variables|Default|SetOn_Off true))

(event EventTick
  (params (DeltaSeconds :type Float%20%28single-precision%29))
  (if (Variables|Default|GetOn_Off)
    (Utilities|FlowControl|DoOnce false :!label _label
      (:Completed
        (Utilities|FlowControl|Delay (Math|Random|RandomFloatinRange (Variables|Default|GetMinBlinkTime) (Variables|Default|GetMaxBlinkTime)))
        (Utilities|FlowControl|FlipFlop
          (:A
            (Rendering|SetVisibility (Variables|Default|GetSpotLight) true false)
            (Rendering|Material|SetMaterial (Variables|Default|GetStaticMesh) 0 (Variables|Default|GetOnMAT))
            (goto _label Reset))
          (:B
            (Rendering|SetVisibility (Variables|Default|GetSpotLight) false false)
            (Rendering|Material|SetMaterial (Variables|Default|GetStaticMesh) 0 (Variables|Default|GetOffMAT))
            (goto _label Reset)))))))

(event EventBeginPlay
  (Variables|Default|GetOnMAT
    (:then
      (bind _offmat (Variables|Default|GetOffMAT)
        (:then
          (Rendering|Material|SetMaterial (Variables|Default|GetStaticMesh) 0 _offmat))
        (:else
          (bind _returnvalue (Rendering|Material|CreateDynamicMaterialInstance (Variables|Default|GetStaticMesh) 0 "/Game/PropsFBX/Fluorescente/FluorescenteApagado_Inst.FluorescenteApagado_Inst" "None" :!class /Script/Engine.PrimitiveComponent))
          (bind _output_get (Variables|Default|SetOffMAT _returnvalue))
          (Rendering|Material|SetMaterial (Variables|Default|GetStaticMesh) 0 _output_get))))
    (:else
      (bind _returnvalue_2 (Rendering|Material|CreateDynamicMaterialInstance (Variables|Default|GetStaticMesh) 0 "/Game/PropsFBX/Fluorescente/FluorescenteEncendido_Inst.FluorescenteEncendido_Inst" "None" :!class /Script/Engine.PrimitiveComponent))
      (Variables|Default|SetOnMAT _returnvalue_2)
      (bind _offmat_2 (Variables|Default|GetOffMAT)
        (:then
          (Rendering|Material|SetMaterial (Variables|Default|GetStaticMesh) 0 _offmat_2))
        (:else
          (bind _returnvalue_3 (Rendering|Material|CreateDynamicMaterialInstance (Variables|Default|GetStaticMesh) 0 "/Game/PropsFBX/Fluorescente/FluorescenteApagado_Inst.FluorescenteApagado_Inst" "None" :!class /Script/Engine.PrimitiveComponent))
          (bind _output_get_2 (Variables|Default|SetOffMAT _returnvalue_3))
          (Rendering|Material|SetMaterial (Variables|Default|GetStaticMesh) 0 _output_get_2))))))

(fn ConstructionScript
  (Rendering|Components|Light|SetIntensity (Variables|Default|GetSpotLight) (Variables|Default|GetLightStrength))
  (if (Variables|Default|GetOn_Off)
    (Rendering|SetVisibility (Variables|Default|GetSpotLight) true false)
    (bind _returnvalue (Rendering|Material|CreateDynamicMaterialInstance (Variables|Default|GetStaticMesh) 0 "/Game/PropsFBX/Fluorescente/FluorescenteEncendido_Inst.FluorescenteEncendido_Inst" "None" :!class /Script/Engine.PrimitiveComponent))
    (Variables|Default|SetOnMAT _returnvalue)
    (else
      (Rendering|SetVisibility (Variables|Default|GetSpotLight) false false)
      (bind _returnvalue_2 (Rendering|Material|CreateDynamicMaterialInstance (Variables|Default|GetStaticMesh) 0 "/Game/PropsFBX/Fluorescente/FluorescenteApagado_Inst.FluorescenteApagado_Inst" "None" :!class /Script/Engine.PrimitiveComponent))
      (Variables|Default|SetOffMAT _returnvalue_2))))