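; Event manager that runs a command-based vote to pick a direction.
; On BeginPlay it registers itself in HODGameInstance and calls DirectionEvent there; starting a direction event clears votes and loads the Direction command list.
; Received commands found in that list add weight at the matching vote index, with commands flagged FromMyself counting far more.
; GetDirectionWinner maps the highest tally's index to one of two enum values.
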(event Custom|StartEvent
  (params (Type :type EventTypes%20Enum :default "NewEnumerator0"))
  ;[1 1 1] StartEvents
  (switch Utilities|FlowControl|Switch|SwitchonEventTypes Type
    (:NewEnumerator0
      (CallFunction|StartDirectionEvent))))

(event Custom|StartDirectionEvent
  ;[1 1 1] StartDirection
  (Utilities|Array|Clear (Variables|Default|GetVotes))
  (Variables|Default|SetActualEvent (Variables|Default|GetDirection)))

(event Custom|ReciveCommand
  (params (Command :type String) (FromMyself :type Boolean))
  (bind _votes (Variables|Default|GetVotes))
  (bind _actualevent (Variables|Default|GetActualEvent))
  (bind _votes_2 (Variables|Default|GetVotes))
  (bind _returnvalue (Utilities|Array|FindItem _actualevent Command))
  (bind _output (Utilities|Array|Get(acopy) _votes _returnvalue))
  ;[1 1 1] ReciveCommands
  (if (Utilities|Array|ContainsItem _actualevent Command)
    (if FromMyself
      (Utilities|Array|SetArrayElem _votes_2 _returnvalue (+ _output 20) true)
      (else
        (Utilities|Array|SetArrayElem _votes_2 _returnvalue (+ _output 1) true)))))

(event EventBeginPlay
  (bind _returnvalue (Game|GetGameInstance))
  (bind _ashodgame_instance (Utilities|Casting|CastToHODGameInstance _returnvalue))
  ;[1 1 1] Set in the Game Instance
  (Variables|/Game/HOD_Content/Blueprint/GameInstance/HODGameInstance.HODGameInstance_C|SetEventManager _ashodgame_instance self)
  (Default|DirectionEvent _ashodgame_instance))

(fn ConstructionScript)

(fn GetDirectionWinner
  (return (Utilities|Select :Index (.IndexOfMaxValue (Math|Integer|MaxOfIntArray (Variables|Default|GetVotes))) :Option%200 "NewEnumerator0" :Option%201 "NewEnumerator1")))