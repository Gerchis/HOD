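; HODGameInstance is a game instance that runs a stream-style chat, showing both Twitch and simulated viewer messages.
; Incoming Twitch messages with a user and text go straight to the ChatHUD.
; Generated messages pair a random active user, line and bright color, then go to the ChatHUD and TwitchIntegration.
; Adding viewers raises the count and grows active users from a name pool, removing a separately randomized index each time.
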(event Custom|GenerateGameMessage
  (CallFunction|GetRandomMessage)
  (Default|SendMessage (Variables|Default|GetChatHUD) (Variables|Default|GetOwner) (Variables|Default|GetMessage) (Variables|Default|GetMessageColor))
  (Class|TwitchChat|SendMessage (Variables|Default|GetTwitchIntegration) (Variables|Default|GetMessage)))

(event Custom|AddUsers
  (params (Cuant :type Integer))
  (bind _users (Variables|Default|GetUsers))
  (bind _returnvalue (Utilities|Array|Length _users))
  (bind _returnvalue_2 (Math|Random|RandomInteger _returnvalue))
  (for _index (range 0 Cuant)
    (if (< 0 _returnvalue)
      (Utilities|Array|Add (Variables|Default|GetActualUsers) (Utilities|Array|Get(acopy) _users _returnvalue_2))
      (Utilities|Array|RemoveIndex _users _returnvalue_2))))

(event Custom|AddViewers
  (params (Cuant :type Integer))
  (Variables|Default|SetViewers (+ Cuant (Variables|Default|GetViewers)))
  (CallFunction|AddUsers Cuant))

(event Custom|GenerateTwitchMessage
  (params (User :type String) (Message :type String) (NewParam :type Slate%20Color%20Structure))
  (if (and (Utilities|Enum|NotEqual(Enum) User "") (Utilities|Enum|NotEqual(Enum) Message ""))
    (Default|SendMessage (Variables|Default|GetChatHUD) User Message NewParam)))

(event Custom|GetRandomMessage
  (bind _actualusers (Variables|Default|GetActualUsers))
  (bind _messages (Variables|Default|GetMessages))
  (Variables|Default|SetOwner (Utilities|Array|Get(acopy) _actualusers (Math|Random|RandomInteger (Utilities|Array|Length _actualusers))))
  (Variables|Default|SetMessage (Utilities|Array|Get(acopy) _messages (Math|Random|RandomInteger (Utilities|Array|Length _messages))))
  (Variables|Default|SetMessageColor (Utilities|Struct|MakeSlateColor (Utilities|Struct|MakeLinearColor (Math|Random|RandomFloatinRange 0.5 1.0) (Math|Random|RandomFloatinRange 0.5 1.0) (Math|Random|RandomFloatinRange 0.5 1.0) 1.0))))