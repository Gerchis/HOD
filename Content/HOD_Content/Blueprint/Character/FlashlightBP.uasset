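; Flashlight actor that follows the player's flashlight component and aims where the camera is looking.
; Every tick it moves to the HOD_Player's Flashlight world location, then uses its Linterna component's location while setting rotation.
; Rotation interpolates quickly toward the end point of a camera-forward visibility trace, using the trace end rather than the impact point, so obstacles do not affect the aim.
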(event Custom|MovementFlashlight
  (bind _returnvalue (Game|GetPlayerCameraManager 0))
  (bind _self self)
  (bind _returnvalue_2 (Transformation|GetActorLocation _returnvalue))
  (Transformation|SetActorLocation (Transformation|GetWorldLocation (Variables|/Game/HOD_Content/Blueprint/Character/HOD_Player.HOD_Player_C|GetFlashlight (.AsHOD%20Player (Utilities|Casting|CastToHOD_Player (Game|GetPlayerCharacter 0))))) false false)
  (bind _outhit (Collision|LineTraceByChannel _returnvalue_2 (+ _returnvalue_2 (* (Transformation|GetActorForwardVector _returnvalue) 1024.0)) "TraceTypeQuery1" false 0 "None"))
  (Transformation|SetActorLocationAndRotation (Transformation|GetWorldLocation (Variables|Default|GetLinterna)) (Math|Interpolation|RInterpTo (Transformation|GetActorRotation _self) (Math|Rotator|FindLookatRotation (Transformation|GetActorLocation _self) (.TraceEnd (Collision|BreakHitResult _outhit))) (Utilities|Time|GetWorldDeltaSeconds) 1e+02)))

(event EventTick
  (params (DeltaSeconds :type Float%20%28single-precision%29))
  (CallFunction|MovementFlashlight))

(fn ConstructionScript)