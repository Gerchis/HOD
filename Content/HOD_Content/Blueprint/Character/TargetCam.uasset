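; TargetCam is a target actor that steers the player's view toward its own location.
; On BeginPlay it enables its tick if the HOD_Player's LookAround flag is off.
; Each tick it smoothly interpolates the player controller's control rotation toward a look-at rotation from PlayerCamera to itself, with a 90-degree roll offset added.
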(event EventBeginPlay
  (if (not (Variables|/Game/HOD_Content/Blueprint/Character/HOD_Player.HOD_Player_C|GetLookAround (.AsHOD%20Player (Utilities|Casting|CastToHOD_Player (Game|Player|GetPlayerPawn 0)))))
    (Actor|Tick|SetActorTickEnabled true)))

(event EventTick
  (params (DeltaSeconds :type Float%20%28single-precision%29))
  (bind _returnvalue (Game|Player|GetPlayerPawn 0))
  (bind _returnvalue_2 (Transformation|GetActorLocation))
  (bind _returnvalue_3 (Game|GetPlayerController 0))
  (bind _ashod_player (Utilities|Casting|CastToHOD_Player _returnvalue))
  (bind _playercamera (Variables|/Game/HOD_Content/Blueprint/Character/HOD_Player.HOD_Player_C|GetPlayerCamera _ashod_player))
  (bind _returnvalue_4 (Transformation|GetWorldLocation _playercamera))
  (bind _returnvalue_5 (Math|Rotator|FindLookatRotation _returnvalue_4 _returnvalue_2))
  (bind (_roll _pitch _yaw) (Math|Rotator|BreakRotator _returnvalue_5))
  (Pawn|SetControlRotation _returnvalue_3 (Math|Interpolation|RInterpTo (Pawn|GetControlRotation _returnvalue_3 :!class /Script/Engine.Controller) (Math|Rotator|MakeRotator (+ _roll 9e+01) _pitch _yaw) DeltaSeconds 1.0)))

(fn ConstructionScript)