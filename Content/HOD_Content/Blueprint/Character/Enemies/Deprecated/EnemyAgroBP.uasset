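; Deprecated enemy pawn that chases and attacks the player once they overlap its detection box, stopping active movement when they leave.
; Each successful AI move onto the player triggers a timed attack, then a retreat to the spawn point before chasing again.
; Attacks increment a hit counter that kills the player at five, while a delay on Tick gradually decays it.
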(event OnComponentBeginOverlap(Box)
  (params (OverlappedComponent :type Primitive%20Component%20Object%20Reference) (OtherActor :type Actor%20Object%20Reference) (OtherComp :type Primitive%20Component%20Object%20Reference) (OtherBodyIndex :type Integer) (bFromSweep :type Boolean) (SweepResult :type Hit%20Result%20Structure%20%28by%20ref%29))
  (Utilities|Casting|CastToHOD_Player OtherActor)
  (CallFunction|ChasePlayer))

(event OnComponentEndOverlap(Box)
  (params (OverlappedComponent :type Primitive%20Component%20Object%20Reference) (OtherActor :type Actor%20Object%20Reference) (OtherComp :type Primitive%20Component%20Object%20Reference) (OtherBodyIndex :type Integer))
  (Utilities|Casting|CastToHOD_Player OtherActor)
  (Class|NavMovementComponent|StopActiveMovement (Variables|Default|GetFloatingPawnMovement)))

(event Custom|ChasePlayer
  (bind _returnvalue (Game|Player|GetPlayerPawn 0))
  (bind _ashod_player (Utilities|Casting|CastToHOD_Player _returnvalue))
  (AI|AIMoveTo self (Transformation|GetActorLocation _ashod_player) _ashod_player 1e+01 false
    (:OnSuccess
      (CallFunction|Attack))
    (:OnFail
      (Development|PrintString "Hello"))))

(event Custom|Attack
  (bind _hitsdone (Variables|Default|GetHitsDone))
  (Variables|Default|SetAttacking true)
  (Utilities|FlowControl|Delay (Variables|Default|GetAttackAnimDuration))
  (Variables|Default|SetAttacking false)
  (Math|Float|IncrementFloat _hitsdone
    (:%20%20
      (if (>= _hitsdone 5.0)
        (Default|DiebyDamage (.AsHOD%20Player (Utilities|Casting|CastToHOD_Player (Game|GetPlayerCharacter 0))))
        (else
          (CallFunction|Return))))))

(event Custom|Return
  (AI|AIMoveTo self (Variables|Default|GetStarterPoint) 0 5.0 false
    (:OnSuccess
      (CallFunction|ChasePlayer))))

(event EventTick
  (params (DeltaSeconds :type Float%20%28single-precision%29))
  (if (> (Variables|Default|GetHitsDone) 0.0)
    (Utilities|FlowControl|Delay 8.5)
    (Math|Float|DecrementFloat (Variables|Default|GetHitsDone))))

(event EventBeginPlay
  (Variables|Default|SetStarterPoint (Transformation|GetActorLocation)))

(fn ConstructionScript)