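; EnemyLibraryBP is a library enemy that chases the player and attacks on reaching them.
; A player overlapping its Box starts a single AI move toward the player pawn.
; A successful move sets the Attacking flag, while a failed one only prints a debug message.
; It records its spawn location in StarterPoint on BeginPlay, though this graph never uses it.
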(event OnComponentBeginOverlap(Box)
  (params (OverlappedComponent :type Primitive%20Component%20Object%20Reference) (OtherActor :type Actor%20Object%20Reference) (OtherComp :type Primitive%20Component%20Object%20Reference) (OtherBodyIndex :type Integer) (bFromSweep :type Boolean) (SweepResult :type Hit%20Result%20Structure%20%28by%20ref%29))
  (Utilities|Casting|CastToHOD_Player OtherActor)
  (CallFunction|ChasePlayer))

(event Custom|ChasePlayer
  (bind _returnvalue (Game|Player|GetPlayerPawn 0))
  (bind _ashod_player (Utilities|Casting|CastToHOD_Player _returnvalue))
  (AI|AIMoveTo self (Transformation|GetActorLocation _ashod_player) _ashod_player 5e+01 false
    (:OnSuccess
      (CallFunction|Attack))
    (:OnFail
      (Development|PrintString "FailChase"))))

(event Custom|Attack
  (Variables|Default|SetAttacking true))

(event EventTick
  (params (DeltaSeconds :type Float%20%28single-precision%29)))

(event EventBeginPlay
  (Variables|Default|SetStarterPoint (Transformation|GetActorLocation)))

(fn ConstructionScript)