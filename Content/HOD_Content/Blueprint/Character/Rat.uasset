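; Rat character that, on a one-shot Trigger event, appears and runs toward the player, apparently as a scripted scare.
; Trigger unhides it and issues a single SimpleMoveToLocation to player 0's position at that moment, raised by a Z offset, without continuous tracking.
; It also plays a placeholder CompileFailed sound at its location; a TODO notes the offset, sound and trigger-area hookup remain unfinished.
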(event Custom|Trigger
  (bind _returnvalue (Game|Player|GetPlayerPawn 0))
  (bind _returnvalue_2 (Transformation|GetActorLocation _returnvalue))
  (bind (_x _y _z) (Math|Vector|BreakVector _returnvalue_2))
  ;[1 0 1] TODO: Adjust PlayerLocationzOffset (or change it to Y or X if needed) to make it fit as what we want in the game, put the correct sound and call this function when you actually reach the trigger area.
  (if (not (Variables|Default|GetTriggered))
    (Variables|Default|SetTriggered true)
    (Rendering|SetActorHiddenInGame false)
    (AI|Navigation|SimpleMovetoLocation (Pawn|GetController) (Math|Vector|MakeVector _x _y (+ _z (Variables|Default|GetPlayerLocationZOffset))))
    (Audio|PlaySoundatLocation "/Engine/EditorSounds/Notifications/CompileFailed.CompileFailed" (Transformation|GetActorLocation) "0, 0, 0" 1.0 1.0 0.0 0 0 0)))

(fn ConstructionScript)