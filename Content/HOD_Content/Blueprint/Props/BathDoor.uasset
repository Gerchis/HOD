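; BathDoor is a bathroom door prop that swings open physically when pushed.
; PushDoor plays a metal door sound at the actor and turns on physics simulation on RootPuerta.
; It applies a forward force scaled by the Force variable, then disables simulation after a short delay to freeze the door in place.
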(event Custom|PushDoor
  (bind _rootpuerta (Variables|Default|GetRootPuerta))
  (Audio|PlaySoundatLocation "/Game/HOD_Content/Sounds/Doors/MetalDoor.MetalDoor" (Transformation|GetActorLocation) "0, 0, 0" 1.0 1.0 0.0 0 0 0)
  (Physics|SetSimulatePhysics _rootpuerta true)
  (Physics|AddForce _rootpuerta (* (Transformation|GetActorForwardVector) (Variables|Default|GetForce)) "None" false)
  (Utilities|FlowControl|Delay 1.5)
  (Physics|SetSimulatePhysics (Variables|Default|GetRootPuerta) false))

(fn ConstructionScript)