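; PhoneBP is a phone prop the player picks up, which opens the fullscreen chat UI.
; While visible, its Interaction overlap registers it as the HOD_Player's Interact target and toggles a glow on its mesh.
; Interacting calls an extra event, plays a sound, shows the GameInstance's ChatFullscreen widget with its GetMobile animation, then destroys the actor.
; An Appear event makes the mesh visible and enables these interactions.
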(event OnComponentBeginOverlap(Interaction)
  (params (OverlappedComponent :type Primitive%20Component%20Object%20Reference) (OtherActor :type Actor%20Object%20Reference) (OtherComp :type Primitive%20Component%20Object%20Reference) (OtherBodyIndex :type Integer) (bFromSweep :type Boolean) (SweepResult :type Hit%20Result%20Structure%20%28by%20ref%29))
  (if (Variables|Default|GetIsVisible)
    (bind _ashod_player (Utilities|Casting|CastToHOD_Player OtherActor))
    (Variables|/Game/HOD_Content/Blueprint/Character/HOD_Player.HOD_Player_C|SetInteract _ashod_player self)
    (Default|ActivateGlow _ashod_player (Utilities|Array|MakeArray (Variables|Default|GetStaticMesh)))))

(event OnComponentEndOverlap(Interaction)
  (params (OverlappedComponent :type Primitive%20Component%20Object%20Reference) (OtherActor :type Actor%20Object%20Reference) (OtherComp :type Primitive%20Component%20Object%20Reference) (OtherBodyIndex :type Integer))
  (if (Variables|Default|GetIsVisible)
    (bind _ashod_player (Utilities|Casting|CastToHOD_Player OtherActor))
    (Default|DesactivateGlow _ashod_player (Utilities|Array|MakeArray (Variables|Default|GetStaticMesh)))))

(event Custom|Appear
  (Rendering|SetVisibility (Variables|Default|GetStaticMesh) true false)
  (Variables|Default|SetIsVisible true))

(event EventInteractwithActor
  (bind _returnvalue (Game|GetGameInstance))
  (bind _ashodgame_instance (Utilities|Casting|CastToHODGameInstance _returnvalue))
  (bind _chatfullscreen (Variables|/Game/HOD_Content/Blueprint/GameInstance/HODGameInstance.HODGameInstance_C|GetChatFullscreen _ashodgame_instance))
  (if (Variables|Default|GetIsVisible)
    (Default|CallExtraEvent)
    (Audio|PlaySoundatLocation 0 (Transformation|GetActorLocation) "0, 0, 0" 1.0 1.0 0.0 0 0 0)
    (UserInterface|Viewport|AddtoViewport _chatfullscreen 0)
    (UserInterface|Animation|PlayAnimation _chatfullscreen (Variables|/Game/HOD_Content/Blueprint/ChatHUD/FullscreenGame.FullscreenGame_C|GetGetMobile _chatfullscreen) 0.0 1 "Forward" 1.0 false)
    (Actor|DestroyActor)))

(fn ConstructionScript)