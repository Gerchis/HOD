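; Lab detector prop, apparently a keycard reader, that opens the linked elevator's doors once the Tarjeta (card) reference is no longer valid.
; Box overlap registers it as the HOD_Player's interact target and toggles the mesh glow; leaving does not clear that target.
; Interacting plays a failure sound while the card exists, otherwise a success sound, swaps the material, zeroes custom depth stencil and calls AbrirPuertas on Ascensor.
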(event OnComponentBeginOverlap(Box)
  (params (OverlappedComponent :type Primitive%20Component%20Object%20Reference) (OtherActor :type Actor%20Object%20Reference) (OtherComp :type Primitive%20Component%20Object%20Reference) (OtherBodyIndex :type Integer) (bFromSweep :type Boolean) (SweepResult :type Hit%20Result%20Structure%20%28by%20ref%29))
  (bind _ashod_player (Utilities|Casting|CastToHOD_Player OtherActor))
  (Variables|/Game/HOD_Content/Blueprint/Character/HOD_Player.HOD_Player_C|SetInteract _ashod_player self)
  (Default|ActivateGlow _ashod_player (Utilities|Array|MakeArray (Variables|Default|GetStaticMesh))))

(event OnComponentEndOverlap(Box)
  (params (OverlappedComponent :type Primitive%20Component%20Object%20Reference) (OtherActor :type Actor%20Object%20Reference) (OtherComp :type Primitive%20Component%20Object%20Reference) (OtherBodyIndex :type Integer))
  (bind _ashod_player (Utilities|Casting|CastToHOD_Player OtherActor))
  (Default|DesactivateGlow _ashod_player (Utilities|Array|MakeArray (Variables|Default|GetStaticMesh))))

(event EventInteractwithActor
  (bind _staticmesh (Variables|Default|GetStaticMesh))
  (Variables|Default|GetTarjeta
    (:then
      (Audio|PlaySound2D "/Engine/EditorSounds/Notifications/CompileFailed.CompileFailed" 1.0 1.0 0.0 0 0)
      (Utilities|FlowControl|DoOnce false))
    (:else
      (Audio|PlaySound2D "/Engine/EditorSounds/Notifications/CompileSuccess.CompileSuccess" 1.0 1.0 0.0 0 0)
      (Rendering|Material|SetMaterial _staticmesh 0 (Variables|Default|GetActivateMaterial))
      (Rendering|SetCustomDepthStencilValue _staticmesh 0)
      (Default|AbrirPuertas (Variables|Default|GetAscensor)))))

(fn ConstructionScript)