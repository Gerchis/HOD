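; Interactable hinged door that creaks open and shut, and stays locked with a rattle animation while a required DoorKey is still valid.
; Overlapping Detection registers the door as the HOD_Player's interact target and makes both handles glow.
; Interacting alternates playing and reversing a rotation timeline, with three line traces checking for the player to choose the swing side.
; A DoOnce holds that side until closing finishes.
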(event OnComponentEndOverlap(Detection)
  (params (OverlappedComponent :type Primitive%20Component%20Object%20Reference) (OtherActor :type Actor%20Object%20Reference) (OtherComp :type Primitive%20Component%20Object%20Reference) (OtherBodyIndex :type Integer))
  (bind _ashod_player (Utilities|Casting|CastToHOD_Player OtherActor))
  (Default|DesactivateGlow _ashod_player (Utilities|Array|MakeArray (Variables|Default|GetHandle) (Variables|Default|GetHandle1))))

(event OnComponentBeginOverlap(Detection)
  (params (OverlappedComponent :type Primitive%20Component%20Object%20Reference) (OtherActor :type Actor%20Object%20Reference) (OtherComp :type Primitive%20Component%20Object%20Reference) (OtherBodyIndex :type Integer) (bFromSweep :type Boolean) (SweepResult :type Hit%20Result%20Structure%20%28by%20ref%29))
  (bind _ashod_player (Utilities|Casting|CastToHOD_Player OtherActor))
  (Variables|/Game/HOD_Content/Blueprint/Character/HOD_Player.HOD_Player_C|SetInteract _ashod_player self)
  (Default|ActivateGlow _ashod_player (Utilities|Array|MakeArray (Variables|Default|GetHandle) (Variables|Default|GetHandle1))))

(event Custom|SetIfCasted
  (params (Casted :type Boolean))
  (Utilities|FlowControl|DoOnce false
    (:Completed
      (Variables|Default|SetCasted Casted))))

(event EventInteractwithActor
  (bind _raycastspawner1 (Variables|Default|GetRaycastSpawner1))
  (bind _raycastspawner2 (Variables|Default|GetRaycastSpawner2))
  (bind _raycastspawner (Variables|Default|GetRaycastSpawner))
  (bind _returnvalue (Transformation|GetWorldLocation _raycastspawner1))
  (bind _returnvalue_2 (Transformation|GetWorldLocation _raycastspawner2))
  (bind _returnvalue_3 (Transformation|GetWorldLocation _raycastspawner))
  (if (Variables|Default|GetOpen)
    (Variables|Default|SetOpen false)
    (bind _returnvalue_4 (Audio|SpawnSoundAttached "/Game/HOD_Content/Sounds/Doors/Door_Creepy_Open_03.Door_Creepy_Open_03" (Variables|Default|GetDoorRotate) "None" "0, 0, 0" "0, 0, 0" "KeepRelativeOffset" false 1.0 1.0 0.0 0 0))
    (bind _outhit (Collision|LineTraceByChannel _returnvalue_3 (- (* _returnvalue_3 (Transformation|GetActorForwardVector)) "0.000000,0.000000,-850.000000") "TraceTypeQuery1" false 0 "ForDuration" :!label _label))
    (bind _outhit_2 (Collision|LineTraceByChannel _returnvalue (- (* _returnvalue (Transformation|GetActorForwardVector)) "0.000000,0.000000,-850.000000") "TraceTypeQuery1" false 0 "ForDuration"))
    (bind _outhit_3 (Collision|LineTraceByChannel _returnvalue_2 (- (* _returnvalue_2 (Transformation|GetActorForwardVector)) "0.000000,0.000000,-850.000000") "TraceTypeQuery1" false 0 "ForDuration"))
    (Utilities|FlowControl|FlipFlop
      (:A
        (Utilities|Casting|CastToHOD_Player (.HitActor (Collision|BreakHitResult _outhit))
          (:then
            (CallFunction|SetifCasted true :!label _label_2)
            (Variables|Default|SetClosing false)
            (bind (_direction _opendoor) (Timeline|OpenDoor Play)
              (:Update
                (if (Variables|Default|GetClosing)
                  (if (Variables|Default|GetCasted)
                    (Transformation|SetRelativeRotation (Variables|Default|GetDoorRotate) (Math|Rotator|Lerp(Rotator) "0, 0, 0" "0,-80.000000, 0" _opendoor true) false false :!label _label_3)
                    (else
                      (Transformation|SetRelativeRotation (Variables|Default|GetDoorRotate) (Math|Rotator|Lerp(Rotator) "0, 0, 0" "0,80.000000, 0" _opendoor true) false false :!label _label_4)))
                  (elif (Variables|Default|GetCasted)
                    (goto _label_3)
                    (else
                      (goto _label_4)))))
              (:Finished
                (if (Variables|Default|GetClosing)
                  (Utilities|FlowControl|Sequence
                    (:then_0
                      (switch Utilities|FlowControl|Switch|SwitchonETimelineDirection _direction :!label _label_5
                        (:Backward
                          (Audio|SpawnSoundAttached "/Game/NinaTemplate/NinaTemplate/GeneralBlueprints/NinaFirstPerson/GenericInteracts/Doors/Sounds/Door_close_12.Door_close_12" (Variables|Default|GetDoorRotate) "None" "0, 0, 0" "0, 0, 0" "KeepRelativeOffset" false 1.0 1.0 0.0 0 0)
                          (if (Audio|Components|Audio|IsPlaying _returnvalue_4)
                            (Audio|Components|Audio|Stop _returnvalue_4)))))
                    (:then_1
                      (Utilities|FlowControl|DoOnce false) ; enters at Reset
                    ))
                  (else
                    (goto _label_5))))))
          (:CastFailed
            (Utilities|Casting|CastToHOD_Player (.HitActor (Collision|BreakHitResult _outhit_2))
              (:then
                (goto _label_2))
              (:CastFailed
                (Utilities|Casting|CastToHOD_Player (.HitActor (Collision|BreakHitResult _outhit_3))
                  (:then
                    (goto _label_2))
                  (:CastFailed
                    (CallFunction|SetifCasted false)
                    (Variables|Default|SetClosing false)
                    (Timeline|OpenDoor Play))))))))
      (:B
        (Utilities|Casting|CastToHOD_Player (.HitActor (Collision|BreakHitResult _outhit))
          (:then
            (CallFunction|SetifCasted true :!label _label_6)
            (Variables|Default|SetClosing true)
            (Timeline|OpenDoor Reverse))
          (:CastFailed
            (Utilities|Casting|CastToHOD_Player (.HitActor (Collision|BreakHitResult _outhit_2))
              (:then
                (goto _label_6))
              (:CastFailed
                (Utilities|Casting|CastToHOD_Player (.HitActor (Collision|BreakHitResult _outhit_3))
                  (:then
                    (goto _label_6))
                  (:CastFailed
                    (CallFunction|SetifCasted false)
                    (Variables|Default|SetClosing true)
                    (Timeline|OpenDoor Reverse)))))))))
    (elif (Variables|Default|GetNeedsKey)
      (Utilities|IsValid (Variables|Default|GetDoorKey)
        (:Is%20Valid
          (Audio|SpawnSoundAttached "/Game/HOD_Content/Sounds/Doors/Door_Locked.Door_Locked" (Variables|Default|GetDoorRotate) "None" "0, 0, 0" "0, 0, 0" "KeepRelativeOffset" false 1.0 1.0 0.0 0 0)
          (bind _closeddoor (Timeline|ClosedDoor PlayFromStart)
            (:Update
              (Transformation|SetRelativeRotation (Variables|Default|GetDoorRotate) (Math|Rotator|Lerp(Rotator) "0, 0, 0" "0,80.000000, 0" _closeddoor true) false false))))
        (:Is%20Not%20Valid
          (Variables|Default|SetOpen true :!label _label_7)
          (Audio|SpawnSoundAttached "/Game/HOD_Content/Sounds/Doors/Door_squeak_creak_09.Door_squeak_creak_09" (Variables|Default|GetDoorRotate) "None" "0, 0, 0" "0, 0, 0" "KeepRelativeOffset" false 1.0 1.0 0.0 0 0)
          (goto _label)))
      (else
        (goto _label_7)))))

(fn ConstructionScript)