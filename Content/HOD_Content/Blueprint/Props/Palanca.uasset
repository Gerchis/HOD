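; Palanca is a one-time lever prop that the player pulls to trigger a wall level sequence.
; Box overlap registers it as the player's interactable, makes its Soporte and Palanca parts glow, and opens a gate; leaving reverses the glow and gate.
; InteractwithActor passes that gate and a DoOnce, then plays the sequence, a sound at SoundOrigin, and a timeline that rolls the lever.
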(event OnComponentBeginOverlap(Box)
  (params (OverlappedComponent :type Primitive%20Component%20Object%20Reference) (OtherActor :type Actor%20Object%20Reference) (OtherComp :type Primitive%20Component%20Object%20Reference) (OtherBodyIndex :type Integer) (bFromSweep :type Boolean) (SweepResult :type Hit%20Result%20Structure%20%28by%20ref%29))
  (bind _returnvalue (Game|GetPlayerCharacter 0))
  (bind _palanca (Variables|Default|GetPalanca))
  (bind _returnvalue_2 (Transformation|GetWorldRotation _palanca))
  (bind _ashod_player (Utilities|Casting|CastToHOD_Player _returnvalue))
  (Variables|/Game/HOD_Content/Blueprint/Character/HOD_Player.HOD_Player_C|SetInteract _ashod_player self)
  (Default|ActivateGlow _ashod_player (Utilities|Array|MakeArray (Variables|Default|GetSoporte) (Variables|Default|GetPalanca)))
  (Utilities|Casting|CastToHOD_Player OtherActor)
  (Utilities|FlowControl|Gate true) ; enters at Open
)

(event OnComponentEndOverlap(Box)
  (params (OverlappedComponent :type Primitive%20Component%20Object%20Reference) (OtherActor :type Actor%20Object%20Reference) (OtherComp :type Primitive%20Component%20Object%20Reference) (OtherBodyIndex :type Integer))
  (bind _palanca (Variables|Default|GetPalanca))
  (bind _returnvalue (Transformation|GetWorldRotation _palanca))
  (bind _ashod_player (Utilities|Casting|CastToHOD_Player OtherActor))
  (Default|DesactivateGlow _ashod_player (Utilities|Array|MakeArray (Variables|Default|GetSoporte) (Variables|Default|GetPalanca)))
  (Utilities|FlowControl|Gate true) ; enters at Close
)

(event EventInteractwithActor
  (bind _palanca (Variables|Default|GetPalanca))
  (bind _returnvalue (Transformation|GetWorldRotation _palanca))
  (Utilities|FlowControl|Gate true
    (:Exit
      (Utilities|FlowControl|DoOnce false
        (:Completed
          (bind _returnvalue_2 (Sequencer|Player|CreateLevelSequencePlayer (Variables|Default|GetWallSequence)))
          (Sequencer|Player|Play _returnvalue_2 :!class /Script/MovieScene.MovieSceneSequencePlayer)
          (Audio|PlaySoundatLocation (Variables|Default|GetSound) (Transformation|GetActorLocation (Variables|Default|GetSoundOrigin)) "0, 0, 0" 1.0 1.0 0.0 0 0 0)
          (bind _newtrack_0 (Timeline|PalancaTL Play)
            (:Update
              (Transformation|SetWorldRotation _palanca (Math|Rotator|MakeRotator _newtrack_0 (.pitch _returnvalue) (.yaw _returnvalue)) false false))))))))

(fn ConstructionScript)