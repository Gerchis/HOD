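; Card detector prop that the player interacts with to open the elevator and trigger the boss sequence.
; A box overlap registers it as the player's interact target and toggles its mesh glow.
; While the Tarjeta (card) actor is still valid, interaction plays a failure sound and fires a one-time message event.
; Otherwise it activates, freezes the player, and runs timed door opening, camera shake, player fall and boss event.
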(event OnComponentBeginOverlap(Box)
  (params (OverlappedComponent :type Primitive%20Component%20Object%20Reference) (OtherActor :type Actor%20Object%20Reference) (OtherComp :type Primitive%20Component%20Object%20Reference) (OtherBodyIndex :type Integer) (bFromSweep :type Boolean) (SweepResult :type Hit%20Result%20Structure%20%28by%20ref%29))
  (bind _ashod_player (Utilities|Casting|CastToHOD_Player OtherActor))
  (Variables|/Game/HOD_Content/Blueprint/Character/HOD_Player.HOD_Player_C|SetInteract _ashod_player self)
  (Default|ActivateGlow _ashod_player (Utilities|Array|MakeArray (Variables|Default|GetStaticMesh))))

(event OnComponentEndOverlap(Box)
  (params (OverlappedComponent :type Primitive%20Component%20Object%20Reference) (OtherActor :type Actor%20Object%20Reference) (OtherComp :type Primitive%20Component%20Object%20Reference) (OtherBodyIndex :type Integer))
  (bind _ashod_player (Utilities|Casting|CastToHOD_Player OtherActor))
  (Default|DesactivateGlow _ashod_player (Utilities|Array|MakeArray (Variables|Default|GetStaticMesh))))

(event EventInteractwithActor
  (bind _returnvalue (Game|Player|GetPlayerPawn 0))
  (bind _returnvalue_2 (Game|Player|GetPlayerPawn 0))
  (bind _staticmesh (Variables|Default|GetStaticMesh))
  (bind _ashod_player (Utilities|Casting|CastToHOD_Player _returnvalue))
  (Variables|Default|GetTarjeta
    (:then
      (Audio|PlaySound2D "/Engine/EditorSounds/Notifications/CompileFailed.CompileFailed" 1.0 1.0 0.0 0 0)
      (Utilities|FlowControl|DoOnce false
        (:Completed
          (Default|CallMessageEvent))))
    (:else
      (Audio|PlaySound2D "/Engine/EditorSounds/Notifications/CompileSuccess.CompileSuccess" 1.0 1.0 0.0 0 0)
      (Rendering|Material|SetMaterial _staticmesh 0 (Variables|Default|GetActivateMaterial))
      (Rendering|SetCustomDepthStencilValue _staticmesh 0)
      (Variables|/Game/HOD_Content/Blueprint/Character/HOD_Player.HOD_Player_C|SetCanMove? _ashod_player false)
      (Variables|/Game/HOD_Content/Blueprint/Character/HOD_Player.HOD_Player_C|SetLookAround _ashod_player false)
      (Utilities|FlowControl|Delay 2.0)
      (Default|AbrirPuertas (Variables|Default|GetAscensor))
      (Utilities|FlowControl|Delay 2.0)
      (Camera|PlayWorldCameraShake "/Game/HOD_Content/Blueprint/CameraShake/FinalCameraShake.FinalCameraShake_C" (Transformation|GetActorLocation _returnvalue_2) 1e+02 0.0)
      (Default|Fall (.AsHOD%20Player (Utilities|Casting|CastToHOD_Player _returnvalue_2)))
      (Utilities|FlowControl|Delay 1.0)
      (Default|CallBossEvent))))

(fn ConstructionScript)