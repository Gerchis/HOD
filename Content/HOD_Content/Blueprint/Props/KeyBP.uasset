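; KeyBP is a key prop that the player can interact with, which removes it from the world.
; Overlapping its Interaction component sets the key as the HOD_Player's Interact target and makes the player activate a glow on its StaticMesh.
; Ending the overlap turns the glow off but leaves the Interact reference set.
; The InteractwithActor event only destroys the actor, with no inventory or unlock logic here.
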(event OnComponentBeginOverlap(Interaction)
  (params (OverlappedComponent :type Primitive%20Component%20Object%20Reference) (OtherActor :type Actor%20Object%20Reference) (OtherComp :type Primitive%20Component%20Object%20Reference) (OtherBodyIndex :type Integer) (bFromSweep :type Boolean) (SweepResult :type Hit%20Result%20Structure%20%28by%20ref%29))
  (bind _ashod_player (Utilities|Casting|CastToHOD_Player OtherActor))
  (Variables|/Game/HOD_Content/Blueprint/Character/HOD_Player.HOD_Player_C|SetInteract _ashod_player self)
  (Default|ActivateGlow _ashod_player (Utilities|Array|MakeArray (Variables|Default|GetStaticMesh))))

(event OnComponentEndOverlap(Interaction)
  (params (OverlappedComponent :type Primitive%20Component%20Object%20Reference) (OtherActor :type Actor%20Object%20Reference) (OtherComp :type Primitive%20Component%20Object%20Reference) (OtherBodyIndex :type Integer))
  (bind _ashod_player (Utilities|Casting|CastToHOD_Player OtherActor))
  (Default|DesactivateGlow _ashod_player (Utilities|Array|MakeArray (Variables|Default|GetStaticMesh))))

(event EventInteractwithActor
  (Actor|DestroyActor))

(fn ConstructionScript)