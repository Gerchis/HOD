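; Ladder prop that the player can climb once its linked trapdoor (Trampilla) is open.
; Detection overlap or BO_Ladder registers it as the player's interactable and glows its meshes.
; Interacting toggles climbing through Flying movement and the Escalera flag, entering via a screen blink and a teleport to TP with fixed view rotation.
; Leaving Detection removes the glow, restores Walking and launches the player forward.
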(event OnComponentBeginOverlap(Detection)
  (params (OverlappedComponent :type Primitive%20Component%20Object%20Reference) (OtherActor :type Actor%20Object%20Reference) (OtherComp :type Primitive%20Component%20Object%20Reference) (OtherBodyIndex :type Integer) (bFromSweep :type Boolean) (SweepResult :type Hit%20Result%20Structure%20%28by%20ref%29))
  (bind _ashod_player (Utilities|Casting|CastToHOD_Player OtherActor))
  (if (Variables|/Game/HOD_Content/Blueprint/Props/TrampillaBP.TrampillaBP_C|GetisOpened (Variables|Default|GetTrampilla))
    (Variables|/Game/HOD_Content/Blueprint/Character/HOD_Player.HOD_Player_C|SetInteract _ashod_player self)
    (Default|ActivateGlow _ashod_player (Utilities|Array|MakeArray (Variables|Default|GetStaticMesh) (Variables|Default|GetStaticMesh1) (Variables|Default|GetHierarchicalInstancedStaticMesh)))))

(event OnComponentEndOverlap(Detection)
  (params (OverlappedComponent :type Primitive%20Component%20Object%20Reference) (OtherActor :type Actor%20Object%20Reference) (OtherComp :type Primitive%20Component%20Object%20Reference) (OtherBodyIndex :type Integer))
  (bind _returnvalue (Game|Player|GetPlayerPawn 0))
  (bind _ashod_player (Utilities|Casting|CastToHOD_Player _returnvalue))
  (bind _ashod_player_2 (Utilities|Casting|CastToHOD_Player OtherActor))
  (Default|DesactivateGlow _ashod_player_2 (Utilities|Array|MakeArray (Variables|Default|GetStaticMesh) (Variables|Default|GetStaticMesh1) (Variables|Default|GetHierarchicalInstancedStaticMesh)))
  (Variables|Default|SetUsing false)
  (Pawn|Components|CharacterMovement|SetMovementMode (Variables|/Script/Engine.Character|GetCharacterMovement _ashod_player) "MOVE_Walking" 0)
  (Variables|/Game/HOD_Content/Blueprint/Character/HOD_Player.HOD_Player_C|SetEscalera _ashod_player false)
  (Character|LaunchCharacter _ashod_player (* (Transformation|GetActorForwardVector _ashod_player) (Variables|Default|GetForce)) false false))

(event Custom|BO_Ladder
  (bind _returnvalue (Game|Player|GetPlayerPawn 0))
  (bind _ashod_player (Utilities|Casting|CastToHOD_Player _returnvalue))
  (Variables|/Game/HOD_Content/Blueprint/Character/HOD_Player.HOD_Player_C|SetInteract _ashod_player self)
  (Default|ActivateGlow _ashod_player (Utilities|Array|MakeArray (Variables|Default|GetStaticMesh) (Variables|Default|GetStaticMesh1) (Variables|Default|GetHierarchicalInstancedStaticMesh))))

(event EventInteractwithActor
  (bind _returnvalue (Game|Player|GetPlayerPawn 0))
  (bind _returnvalue_2 (Game|GetGameInstance))
  (bind _returnvalue_3 (Game|Player|GetPlayerPawn 0))
  (bind _ashodgame_instance (Utilities|Casting|CastToHODGameInstance _returnvalue_2))
  (bind _ashod_player (Utilities|Casting|CastToHOD_Player _returnvalue_3))
  (bind _ashod_player_2 (Utilities|Casting|CastToHOD_Player _returnvalue))
  (bind _chatfullscreen (Variables|/Game/HOD_Content/Blueprint/GameInstance/HODGameInstance.HODGameInstance_C|GetChatFullscreen _ashodgame_instance))
  (bind _blink (Variables|/Game/HOD_Content/Blueprint/ChatHUD/FullscreenGame.FullscreenGame_C|GetBlink _chatfullscreen))
  (if (Variables|/Game/HOD_Content/Blueprint/Props/TrampillaBP.TrampillaBP_C|GetisOpened (Variables|Default|GetTrampilla))
    (if (Variables|Default|GetUsing)
      (Variables|Default|SetUsing false)
      (Pawn|Components|CharacterMovement|SetMovementMode (Variables|/Script/Engine.Character|GetCharacterMovement _ashod_player) "MOVE_Walking" 0)
      (Variables|/Game/HOD_Content/Blueprint/Character/HOD_Player.HOD_Player_C|SetEscalera _ashod_player false)
      (else
        (UserInterface|Animation|PlayAnimation _chatfullscreen _blink 0.0 1 "Forward" 1.0 false)
        (Utilities|FlowControl|Delay (/ (Class|WidgetAnimation|GetEndTime _blink) 2.0))
        (Transformation|SetActorLocation _ashod_player_2 (Transformation|GetWorldLocation (Variables|Default|GetTP)) false true)
        (Pawn|SetControlRotation (Game|GetPlayerController 0) (Math|Rotator|MakeRotator 0.0 0.0 -9e+01))
        (Variables|Default|SetUsing true)
        (Pawn|Components|CharacterMovement|SetMovementMode (Variables|/Script/Engine.Character|GetCharacterMovement (.AsHOD%20Player (Utilities|Casting|CastToHOD_Player (Game|Player|GetPlayerPawn 0)))) "MOVE_Flying" 0)
        (Variables|/Game/HOD_Content/Blueprint/Character/HOD_Player.HOD_Player_C|SetEscalera _ashod_player_2 true)))))

(fn ConstructionScript)