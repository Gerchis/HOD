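; TrampillaBP is an interactable trapdoor prop that opens once when interacted with.
; Overlapping its Detection component sets it as the HOD_Player's interact target and makes the Trampilla component glow, while leaving removes only the glow.
; Interaction is guarded by an IsOpened flag and a DoOnce, then plays the TrampillaAnim level sequence and a sound at the trapdoor's location.
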(event OnComponentBeginOverlap(Detection)
  (params (OverlappedComponent :type Primitive%20Component%20Object%20Reference) (OtherActor :type Actor%20Object%20Reference) (OtherComp :type Primitive%20Component%20Object%20Reference) (OtherBodyIndex :type Integer) (bFromSweep :type Boolean) (SweepResult :type Hit%20Result%20Structure%20%28by%20ref%29))
  (bind _ashod_player (Utilities|Casting|CastToHOD_Player OtherActor))
  (Variables|/Game/HOD_Content/Blueprint/Character/HOD_Player.HOD_Player_C|SetInteract _ashod_player self)
  (Default|ActivateGlow _ashod_player (Utilities|Array|MakeArray (Variables|Default|GetTrampilla))))

(event OnComponentEndOverlap(Detection)
  (params (OverlappedComponent :type Primitive%20Component%20Object%20Reference) (OtherActor :type Actor%20Object%20Reference) (OtherComp :type Primitive%20Component%20Object%20Reference) (OtherBodyIndex :type Integer))
  (bind _ashod_player (Utilities|Casting|CastToHOD_Player OtherActor))
  (Default|DesactivateGlow _ashod_player (Utilities|Array|MakeArray (Variables|Default|GetTrampilla))))

(event EventInteractwithActor
  (if (not (Variables|Default|GetisOpened))
    (Variables|Default|SetisOpened true)
    (Utilities|FlowControl|DoOnce false
      (:Completed
        (bind _returnvalue (Sequencer|Player|CreateLevelSequencePlayer (Variables|Default|GetTrampillaAnim)))
        (Sequencer|Player|Play _returnvalue :!class /Script/MovieScene.MovieSceneSequencePlayer)
        (Audio|PlaySoundatLocation (Variables|Default|GetTrampillaSound) (Transformation|GetWorldLocation (Variables|Default|GetTrampilla)) "0, 0, 0" 1.0 1.0 0.0 0 0 0)))))

(fn ConstructionScript)