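; A reusable box trigger Blueprint that fires activation and end-overlap dispatchers, with a configurable extent and text label set at construction.
; Begin overlap checks the actor against a list of tags and, when enabled, fires the dispatcher, optionally once until ResetDoOnce, playing a 2D sound if configured.
; End overlap dispatches without tag or enabled checks.
; Events enable or disable the trigger and fade out its sound.
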(event OnComponentBeginOverlap(Box)
  (params (OverlappedComponent :type Primitive%20Component%20Object%20Reference) (OtherActor :type Actor%20Object%20Reference) (OtherComp :type Primitive%20Component%20Object%20Reference) (OtherBodyIndex :type Integer) (bFromSweep :type Boolean) (SweepResult :type Hit%20Result%20Structure%20%28by%20ref%29))
  (Variables|Default|SetActorHasCorrectTag false)
  (for _array_element (Variables|Default|GetActorHasTagToActivate)
    (if (Actor|ActorHasTag OtherActor _array_element)
      (Variables|Default|SetActorHasCorrectTag true)))
  (if (Variables|Default|GetActorHasCorrectTag)
    (if (Variables|Default|GetEnabled)
      (if (Variables|Default|GetDoOnce)
        (Utilities|FlowControl|DoOnce false
          (:Completed
            _)))
      (Default|CallPerfectTriggerActivatedDispatchers)
      (if (Variables|Default|GetSoundActivated)
        (bind _returnvalue (Audio|SpawnSound2D (Variables|Default|GetSoundToPlay) 1.0 1.0 0.0 0))
        (Variables|Default|SetPlaySound _returnvalue)))))

(event OnComponentEndOverlap(Box)
  (params (OverlappedComponent :type Primitive%20Component%20Object%20Reference) (OtherActor :type Actor%20Object%20Reference) (OtherComp :type Primitive%20Component%20Object%20Reference) (OtherBodyIndex :type Integer))
  (if (Variables|Default|GetDoOnce)
    (Utilities|FlowControl|DoOnce false
      (:Completed
        _)))
  (Default|CallPerfectTriggerEndOverlapDispatcher))

(event Custom|EnableTrigger
  (Variables|Default|SetEnabled true))

(event Custom|DesableTrigger
  (Variables|Default|SetEnabled false))

(event Custom|SoundOff
  (Audio|Components|Audio|FadeOut (Variables|Default|GetPlaySound) 2.0 0.0 "Linear" :!class /Script/Engine.AudioComponent))

(event Custom|ResetDoOnce
  (Utilities|FlowControl|DoOnce false) ; enters at Reset
)

(fn ConstructionScript
  (Components|Box|SetBoxExtent (Variables|Default|GetBox) (Variables|Default|GetTriggerExtent) true)
  (Rendering|Components|TextRender|SetText (Variables|Default|GetTextRender) (Variables|Default|GetTriggerText)))