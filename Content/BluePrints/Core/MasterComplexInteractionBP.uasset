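; Reusable child-actor interaction component that adds player-proximity glow, HUD prompts and an interact callback to its parent actor.
; CustomConstructionScript sizes the glow box and look-at sphere from InteractStructure and collects parent static meshes by name for Custom Depth outlining.
; ComplexInteract sends ComplexInteractMessage to the parent, optionally only once, disabling glow, sphere collision and interaction until re-enabled.
; A resettable DoOnce gates the HUD message and sound.
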(event OnComponentBeginOverlap(Box)
  (params (OverlappedComponent :type Primitive%20Component%20Object%20Reference) (OtherActor :type Actor%20Object%20Reference) (OtherComp :type Primitive%20Component%20Object%20Reference) (OtherBodyIndex :type Integer) (bFromSweep :type Boolean) (SweepResult :type Hit%20Result%20Structure%20%28by%20ref%29))
  (if (Actor|ActorHasTag OtherActor "Player")
    (if (.InteractionEnabled (Utilities|Struct|BreakComplexLookAtInteractStructure (Variables|Default|GetInteractStructure)))
      (CallFunction|BeginGlow))))

(event OnComponentEndOverlap(Box)
  (params (OverlappedComponent :type Primitive%20Component%20Object%20Reference) (OtherActor :type Actor%20Object%20Reference) (OtherComp :type Primitive%20Component%20Object%20Reference) (OtherBodyIndex :type Integer))
  (if (Actor|ActorHasTag OtherActor "Player")
    (if (.InteractionEnabled (Utilities|Struct|BreakComplexLookAtInteractStructure (Variables|Default|GetInteractStructure)))
      (CallFunction|EndGlow))))

(event Custom|ShowInteractMessage
  (bind _interactstructure (Variables|Default|GetInteractStructure))
  (bind (_interactionenabled _doonce _glowoutlinetriggerextents _lookattriggerradius _glowparentcomponentname _interacttext _interactiontodotext _holdtointeract _showmessagesound) (Utilities|Struct|BreakComplexLookAtInteractStructure _interactstructure))
  (Utilities|FlowControl|DoOnce false
    (:Completed
      (Default|ShowHUDMessage (Variables|/Game/BluePrints/Core/FirstPersonCharacter.FirstPersonCharacter_C|GetCharacterHUD (.AsFirst%20Person%20Character (Utilities|Casting|CastToFirstPersonCharacter (Game|GetPlayerCharacter 0)))) (Utilities|Text|ToText(String) (Utilities|String|Append _interacttext " | " _interactiontodotext)) _showmessagesound))))

(event Custom|ResetShowMessageDoOnce
  (bind _interactstructure (Variables|Default|GetInteractStructure))
  (bind (_interactionenabled _doonce _glowoutlinetriggerextents _lookattriggerradius _glowparentcomponentname _interacttext _interactiontodotext _holdtointeract _showmessagesound) (Utilities|Struct|BreakComplexLookAtInteractStructure _interactstructure))
  (Utilities|FlowControl|DoOnce false) ; enters at Reset
)

(event Custom|EndGlow
  (for _array_element (Variables|Default|GetGlowingStaticMeshComponent)
    (Rendering|SetRenderCustomDepth _array_element false)))

(event Custom|BeginGlow
  (for _array_element (Variables|Default|GetGlowingStaticMeshComponent)
    (Rendering|SetRenderCustomDepth _array_element true)))

(event Custom|EnableInteractionAgain
  (CallFunction|ResetDoOnceInteract)
  (Collision|SetCollisionEnabled (Variables|Default|GetSphere) "QueryAndPhysics")
  (Utilities|Struct|SetmembersinComplexLookAtInteractStructure (Variables|Default|GetInteractStructure) true))

(event Custom|ResetDoOnceInteract
  (Utilities|FlowControl|DoOnce false) ; enters at Reset
)

(event EventComplexInteract
  (bind _interactstructure (Variables|Default|GetInteractStructure))
  (bind (_interactionenabled _doonce) (Utilities|Struct|BreakComplexLookAtInteractStructure _interactstructure))
  (if _interactionenabled
    (if _doonce
      (Utilities|FlowControl|DoOnce false
        (:Completed
          (CallFunction|EndGlow)
          (Collision|SetCollisionEnabled (Variables|Default|GetSphere) "NoCollision")
          (Utilities|Struct|SetmembersinComplexLookAtInteractStructure (Variables|Default|GetInteractStructure) false))))
    (Class|MasterComplexInteractionInterface|ComplexInteract(Message) (Actor|GetParentActor))))

(fn ConstructionScript)

(fn CustomConstructionScript
  (bind _interactstructure (Variables|Default|GetInteractStructure))
  (bind (_interactionenabled _doonce _glowoutlinetriggerextents _lookattriggerradius) (Utilities|Struct|BreakComplexLookAtInteractStructure _interactstructure))
  (Components|Box|SetBoxExtent (Variables|Default|GetBox) _glowoutlinetriggerextents true)
  (Components|Sphere|SetSphereRadius (Variables|Default|GetSphere) _lookattriggerradius true)
  (for _array_element (Actor|GetComponentsByClass (Actor|GetParentActor) "/Script/Engine.StaticMeshComponent")
    (for _array_element_2 (.GlowParentComponentName (Utilities|Struct|BreakComplexLookAtInteractStructure (Variables|Default|GetInteractStructure)))
      (if (Utilities|String|Contains (Utilities|GetDisplayName _array_element) _array_element_2)
        (Utilities|Array|Add (Variables|Default|GetGlowingStaticMeshComponent) _array_element)))))