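; Flashlight actor that follows the first-person player and swings smoothly toward where the camera looks.
; Every tick it snaps to the character's Scene component, then sets its location to that of its Linterna component.
; A camera-forward line trace supplies only its end point, not the impact, as the look-at target.
; RInterpTo eases the rotation toward that point, giving the beam a slight lag behind the view.
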(event Custom|MovementFlashlight
  (bind _returnvalue (Game|GetPlayerCameraManager 0))
  (bind _self self)
  (bind _returnvalue_2 (Transformation|GetActorLocation _returnvalue))
  (Transformation|SetActorLocation (Transformation|GetWorldLocation (Variables|/Game/BluePrints/Core/FirstPersonCharacter.FirstPersonCharacter_C|GetScene (.AsFirst%20Person%20Character (Utilities|Casting|CastToFirstPersonCharacter (Game|GetPlayerCharacter 0))))) false false)
  (bind _outhit (Collision|LineTraceByChannel _returnvalue_2 (+ _returnvalue_2 (* (Transformation|GetActorForwardVector _returnvalue) 1024.0)) "TraceTypeQuery1" false 0 "None"))
  (Transformation|SetActorLocationAndRotation (Transformation|GetWorldLocation (Variables|Default|GetLinterna)) (Math|Interpolation|RInterpTo (Transformation|GetActorRotation _self) (Math|Rotator|FindLookatRotation (Transformation|GetActorLocation _self) (.TraceEnd (Collision|BreakHitResult _outhit))) (Utilities|Time|GetWorldDeltaSeconds) 6.0)))

(event EventTick
  (params (DeltaSeconds :type Float%20%28single-precision%29))
  (CallFunction|MovementFlashlight))

(fn ConstructionScript)