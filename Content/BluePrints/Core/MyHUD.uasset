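; MyHUD sets up the game's UI on BeginPlay, creating the pause menu at a high Z-order, a start-of-game fade-in and the in-game HUD widget.
; ShowPauseMenu uses a FlipFlop to toggle menu visibility, mouse cursor and input mode between game-only and game-and-UI.
; BeginPlay calls it once so the menu starts collapsed with game-only input; it does not pause the game itself.
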(event Custom|ShowPauseMenu
  (bind _returnvalue (Game|GetPlayerController 0))
  (bind _pausemenu (Variables|Default|GetPauseMenu))
  (Utilities|FlowControl|FlipFlop
    (:A
      (Widget|SetVisibility _pausemenu "Collapsed")
      (Input|SetInputModeGameOnly _returnvalue)
      (Variables|/Script/Engine.PlayerController|SetbShowMouseCursor _returnvalue false))
    (:B
      (Widget|SetVisibility _pausemenu "Visible")
      (Input|SetInputModeGameandUI _returnvalue _pausemenu "DoNotLock" true)
      (Variables|/Script/Engine.PlayerController|SetbShowMouseCursor _returnvalue true))))

(event EventBeginPlay
  (Utilities|FlowControl|Sequence
    (:then_0
      (bind _returnvalue (UserInterface|CreateWidget "/Game/BluePrints/Widgets/PauseMenu.PauseMenu_C"))
      (bind _output_get (Variables|Default|SetPauseMenu _returnvalue))
      (UserInterface|Viewport|AddtoViewport _output_get 54)
      (CallFunction|ShowPauseMenu))
    (:then_1
      (bind _returnvalue_2 (UserInterface|CreateWidget "/Game/BluePrints/Widgets/FadeInStartGame.FadeInStartGame_C"))
      (UserInterface|Viewport|AddtoViewport _returnvalue_2 0)
      (Utilities|FlowControl|Delay 0.4))
    (:then_2
      (bind _returnvalue_3 (UserInterface|CreateWidget "/Game/BluePrints/Widgets/HUDGame.HUDGame_C"))
      (UserInterface|Viewport|AddtoViewport _returnvalue_3 0))))

(fn ConstructionScript)