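; Street post clock prop that animates hour and minute hands on two clock faces.
; BeginPlay seeds the time from the system clock or a preset SetTime, depending on UseRealTime.
; Tick advances that time by frame delta rather than re-reading the clock, then converts it to hand roll angles in one-second increments.
; The second pair of hands uses negated angles to mirror the first.
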(event EventBeginPlay
  (if (Variables|Default|GetUseRealTime)
    (Variables|Default|SetTime (Math|DateTime|Now))
    (else
      (Variables|Default|SetTime (Variables|Default|GetSetTime)))))

(event Collision|EventActorBeginOverlap
  (params (OtherActor :type Actor%20Object%20Reference)))

(event EventTick
  (params (DeltaSeconds :type Float%20%28single-precision%29))
  (Variables|Default|SetTime (+ (Variables|Default|GetTime) (Math|Timespan|MakeTimespan 0 0 0 0 (Math|Float|Truncate (* 1000 DeltaSeconds)))))
  (Transformation|SetRelativeRotation (Variables|Default|GetHourHand01) (Math|Rotator|MakeRotator (* (+ (* (+ (* (Class|KismetMathLibrary|GetHour12 (Variables|Default|GetTime)) 6e+01) (Math|Conversions|ToFloat(Integer) (Class|KismetMathLibrary|GetMinute (Variables|Default|GetTime)))) 6e+01) (Math|Conversions|ToFloat(Integer) (Class|KismetMathLibrary|GetSecond (Variables|Default|GetTime)))) -0.008333) 0.0 0.0) false false)
  (Transformation|SetRelativeRotation (Variables|Default|GetMinuteHand01) (Math|Rotator|MakeRotator (* (+ (Math|Conversions|ToFloat(Integer) (Class|KismetMathLibrary|GetSecond (Variables|Default|GetTime))) (* (Class|KismetMathLibrary|GetMinute (Variables|Default|GetTime)) 6e+01)) -0.1) 0.0 0.0) false false)
  (Transformation|SetRelativeRotation (Variables|Default|GetHourHand02) (Math|Rotator|MakeRotator (* (* (+ (* (+ (* (Class|KismetMathLibrary|GetHour12 (Variables|Default|GetTime)) 6e+01) (Math|Conversions|ToFloat(Integer) (Class|KismetMathLibrary|GetMinute (Variables|Default|GetTime)))) 6e+01) (Math|Conversions|ToFloat(Integer) (Class|KismetMathLibrary|GetSecond (Variables|Default|GetTime)))) -0.008333) -1.0) 0.0 0.0) false false)
  (Transformation|SetRelativeRotation (Variables|Default|GetMinuteHand02) (Math|Rotator|MakeRotator (* (* (+ (Math|Conversions|ToFloat(Integer) (Class|KismetMathLibrary|GetSecond (Variables|Default|GetTime))) (* (Class|KismetMathLibrary|GetMinute (Variables|Default|GetTime)) 6e+01)) -0.1) -1.0) 0.0 0.0) false false))

(fn ConstructionScript)