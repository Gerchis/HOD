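; Configurable street light prop for the Old JP street props set, with a spot light and an optional light shaft mesh.
; The construction script creates dynamic material instances to apply paint color, rust level and shaft strength, and sets the spot light intensity.
; An on/off flag toggles the spot light and the lamp material's glow, and the shaft shows only when both it and the light are enabled.
; The event graph has no active logic.
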(event EventBeginPlay)

(event Collision|EventActorBeginOverlap
  (params (OtherActor :type Actor%20Object%20Reference)))

(event EventTick
  (params (DeltaSeconds :type Float%20%28single-precision%29)))

(fn ConstructionScript
  (bind _spotlight (Variables|Default|GetSpotLight))
  (bind _sm_lightshaft (Variables|Default|GetSM_LightShaft))
  (bind _returnvalue (Rendering|Material|CreateDynamicMaterialInstance (Variables|Default|GetSM_LightShaft) 0 "/Game/OldJPStreetProps/Materials/M_Lightshaft_Inst.M_Lightshaft_Inst" "None" :!class /Script/Engine.PrimitiveComponent))
  (Rendering|Material|SetScalarParameterValue _returnvalue "LightStrenght" (Variables|Default|GetLightShaftStrenght) :!class /Script/Engine.MaterialInstanceDynamic)
  (Rendering|Components|Light|SetIntensity (Variables|Default|GetSpotLight) (Variables|Default|GetLightStrenght))
  (bind _returnvalue_2 (Rendering|Material|CreateDynamicMaterialInstance (Variables|Default|GetStaticMesh) 0 "/Game/OldJPStreetProps/Materials/M_Streetlight_Inst.M_Streetlight_Inst" "None" :!class /Script/Engine.PrimitiveComponent))
  (Rendering|Material|SetVectorParameterValue _returnvalue_2 "PaintColor" (Variables|Default|GetColor) :!class /Script/Engine.MaterialInstanceDynamic)
  (Rendering|Material|SetScalarParameterValue _returnvalue_2 "RustLevel" (Variables|Default|GetRustLevel) :!class /Script/Engine.MaterialInstanceDynamic)
  (if (Variables|Default|GetLightON_OFF)
    (Rendering|SetVisibility _spotlight true false)
    (Rendering|Material|SetScalarParameterValue _returnvalue_2 "LightStrenght" 3e+01 :!class /Script/Engine.MaterialInstanceDynamic)
    (if (Variables|Default|GetLightShaft)
      (Rendering|SetVisibility _sm_lightshaft true false)
      (else
        (Rendering|SetVisibility _sm_lightshaft false false :!label _label)))
    (else
      (Rendering|SetVisibility _spotlight false false)
      (Rendering|Material|SetScalarParameterValue _returnvalue_2 "LightStrenght" 0.0 :!class /Script/Engine.MaterialInstanceDynamic)
      (goto _label))))