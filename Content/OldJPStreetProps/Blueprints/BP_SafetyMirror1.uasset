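; BP_SafetyMirror1 is a configurable roadside safety mirror prop, with all of its setup done in the construction script.
; It creates dynamic instances of the safety mirror material on the base mesh and the mirror, driven by rust level and paint color variables.
; Exposed values then offset the arm's height and yaw, yaw the holder and pitch the mirror as local transforms.
; The event graph holds no active logic.
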(event EventBeginPlay)

(event Collision|EventActorBeginOverlap
  (params (OtherActor :type Actor%20Object%20Reference)))

(event EventTick
  (params (DeltaSeconds :type Float%20%28single-precision%29)))

(fn ConstructionScript
  ;[1 1 1] Create material instance and set paint color and rust level
  (bind _returnvalue (Rendering|Material|CreateDynamicMaterialInstance (Variables|Default|GetStaticMesh) 0 "/Game/OldJPStreetProps/Materials/M_SafetyMirror_Inst.M_SafetyMirror_Inst" "None" :!class /Script/Engine.PrimitiveComponent))
  (Rendering|Material|SetScalarParameterValue _returnvalue "RustLevel" (Variables|Default|GetRustLevel) :!class /Script/Engine.MaterialInstanceDynamic)
  (Rendering|Material|SetVectorParameterValue _returnvalue "PaintColor" (Variables|Default|GetColor) :!class /Script/Engine.MaterialInstanceDynamic)
  (bind _returnvalue_2 (Rendering|Material|CreateDynamicMaterialInstance (Variables|Default|GetSM_SafetyM_Mirror) 0 "/Game/OldJPStreetProps/Materials/M_SafetyMirror_Inst.M_SafetyMirror_Inst" "None" :!class /Script/Engine.PrimitiveComponent))
  (Rendering|Material|SetScalarParameterValue _returnvalue_2 "RustLevel" (Variables|Default|GetRustLevel) :!class /Script/Engine.MaterialInstanceDynamic)
  (Rendering|Material|SetVectorParameterValue _returnvalue_2 "PaintColor" (Variables|Default|GetColor) :!class /Script/Engine.MaterialInstanceDynamic)
  ;[1 1 1] Set arm hight and rotation
  (Transformation|AddLocalOffset (Variables|Default|GetSM_SafetyM_arm1) (Math|Vector|MakeVector 0.0 0.0 (Variables|Default|GetMirrorHight)) false false)
  (Transformation|AddLocalRotation (Variables|Default|GetSM_SafetyM_arm1) (Math|Rotator|MakeRotator 0.0 0.0 (Variables|Default|GetArmRotation)) false false)
  ;[1 1 1] Set holder rotation
  (Transformation|AddLocalRotation (Variables|Default|GetSM_SafetyM_Holder) (Math|Rotator|MakeRotator 0.0 0.0 (Variables|Default|GetHolderRotation)) false false)
  ;[1 1 1] Set mirror rotation
  (Transformation|AddLocalRotation (Variables|Default|GetSM_SafetyM_Mirror) (Math|Rotator|MakeRotator 0.0 (Variables|Default|GetMirrorRotation) 0.0) false false))