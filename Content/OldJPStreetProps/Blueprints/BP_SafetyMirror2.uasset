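; BP_SafetyMirror2 is a configurable street prop of a safety mirror with two arms, each with a holder and a mirror.
; The Construction Script creates dynamic instances of M_SafetyMirror_Inst on the base mesh and both mirrors, applying a shared paint color and rust level.
; It then offsets each arm by its height and rotates arms and holders in yaw and mirrors in pitch from per-side variables.
; The event graph has no runtime logic.
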(event EventBeginPlay)

(event Collision|EventActorBeginOverlap
  (params (OtherActor :type Actor%20Object%20Reference)))

(event EventTick
  (params (DeltaSeconds :type Float%20%28single-precision%29)))

(fn ConstructionScript
  ;[1 1 1] Create material instance and set paint color and rustlevel
  (bind _returnvalue (Rendering|Material|CreateDynamicMaterialInstance (Variables|Default|GetStaticMesh) 0 "/Game/OldJPStreetProps/Materials/M_SafetyMirror_Inst.M_SafetyMirror_Inst" "None" :!class /Script/Engine.PrimitiveComponent))
  (Rendering|Material|SetScalarParameterValue _returnvalue "RustLevel" (Variables|Default|GetRustLevel) :!class /Script/Engine.MaterialInstanceDynamic)
  (Rendering|Material|SetVectorParameterValue _returnvalue "PaintColor" (Variables|Default|GetColor) :!class /Script/Engine.MaterialInstanceDynamic)
  (bind _returnvalue_2 (Rendering|Material|CreateDynamicMaterialInstance (Variables|Default|GetSM_SafetyM_Mirror) 0 "/Game/OldJPStreetProps/Materials/M_SafetyMirror_Inst.M_SafetyMirror_Inst" "None" :!class /Script/Engine.PrimitiveComponent))
  (Rendering|Material|SetScalarParameterValue _returnvalue_2 "RustLevel" (Variables|Default|GetRustLevel) :!class /Script/Engine.MaterialInstanceDynamic)
  (Rendering|Material|SetVectorParameterValue _returnvalue_2 "PaintColor" (Variables|Default|GetColor) :!class /Script/Engine.MaterialInstanceDynamic)
  (bind _returnvalue_3 (Rendering|Material|CreateDynamicMaterialInstance (Variables|Default|GetSM_SafetyM_Mirror1) 0 "/Game/OldJPStreetProps/Materials/M_SafetyMirror_Inst.M_SafetyMirror_Inst" "None" :!class /Script/Engine.PrimitiveComponent))
  (Rendering|Material|SetScalarParameterValue _returnvalue_3 "RustLevel" (Variables|Default|GetRustLevel) :!class /Script/Engine.MaterialInstanceDynamic)
  (Rendering|Material|SetVectorParameterValue _returnvalue_3 "PaintColor" (Variables|Default|GetColor) :!class /Script/Engine.MaterialInstanceDynamic)
  ;[1 1 1] Set arm1 hight and rotation
  (Transformation|AddLocalOffset (Variables|Default|GetSM_SafetyM_arm1) (Math|Vector|MakeVector 0.0 0.0 (Variables|Default|GetArm1Hight)) false false)
  (Transformation|AddLocalRotation (Variables|Default|GetSM_SafetyM_arm1) (Math|Rotator|MakeRotator 0.0 0.0 (Variables|Default|GetArm1Rotation)) false false)
  ;[1 1 1] Set holder1 rotation
  (Transformation|AddLocalRotation (Variables|Default|GetSM_SafetyM_Holder) (Math|Rotator|MakeRotator 0.0 0.0 (Variables|Default|GetHolder1Rotation)) false false)
  ;[1 1 1] Set mirror1 rotation
  (Transformation|AddLocalRotation (Variables|Default|GetSM_SafetyM_Mirror) (Math|Rotator|MakeRotator 0.0 (Variables|Default|GetMirror1Rotation) 0.0) false false)
  ;[1 1 1] Set arm2 hight and rotation
  (Transformation|AddLocalOffset (Variables|Default|GetSM_SafetyM_arm2) (Math|Vector|MakeVector 0.0 0.0 (Variables|Default|GetArm2Hight)) false false)
  (Transformation|AddLocalRotation (Variables|Default|GetSM_SafetyM_arm2) (Math|Rotator|MakeRotator 0.0 0.0 (Variables|Default|GetArm2Rotation)) false false)
  ;[1 1 1] Set holder1 rotation
  (Transformation|AddLocalRotation (Variables|Default|GetSM_SafetyM_Holder1) (Math|Rotator|MakeRotator 0.0 0.0 (Variables|Default|GetHolder2Rotation)) false false)
  ;[1 1 1] Set mirror1 rotation
  (Transformation|AddLocalRotation (Variables|Default|GetSM_SafetyM_Mirror1) (Math|Rotator|MakeRotator 0.0 (Variables|Default|GetMirror2Rotation) 0.0) false false))