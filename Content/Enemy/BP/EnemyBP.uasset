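; Enemy pawn Blueprint that chases the player once EnemyActivated is set, polling that flag on a delay until then.
; A self-restarting BeginPlay loop reissues AI MoveTo at short intervals, setting the Attack flag from player distance.
; A successful move forces Attack on, then rechecks a tighter range after a retriggerable delay, while failed moves retry later.
; A DestroyEnemy event removes the actor.
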(event Custom|DestroyEnemy
  (Actor|DestroyActor))

(event EventBeginPlay
  (if (Variables|Default|GetEnemyActivated?) :!label _label
    (AI|AIMoveTo self "0, 0, 0" (Game|GetPlayerCharacter 0) 5.0 false
      (:then
        (Utilities|FlowControl|Delay 0.2)
        (Variables|Default|SetAttack (< (Math|Vector|Distance(Vector) (Transformation|GetActorLocation (Game|GetPlayerCharacter 0)) (Transformation|GetActorLocation self)) 2e+02))
        (goto _label))
      (:OnSuccess
        (Variables|Default|SetAttack true)
        (Utilities|FlowControl|Sequence
          (:then_0
            (goto _label))
          (:then_1
            (Utilities|FlowControl|RetriggerableDelay 2.0)
            (Variables|Default|SetAttack (< (Math|Vector|Distance(Vector) (Transformation|GetActorLocation (Game|GetPlayerCharacter 0)) (Transformation|GetActorLocation self)) 1.5e+02))
            (goto _label))))
      (:OnFail
        _)))
  (Utilities|FlowControl|Delay 1.0)
  (goto _label))

(fn ConstructionScript)